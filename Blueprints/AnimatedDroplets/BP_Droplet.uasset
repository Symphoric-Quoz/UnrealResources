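; BP_Droplet is a single animated droplet that moves itself using settings from its owning simulator.
; Init stores position, direction and size, then picks a first movement behaviour.
; Move delegates to the current mover object and picks a new behaviour whenever that movement finishes.
; Each pick randomises speed and, by a percentage threshold, constructs either a linear mover or a left or right strafe mover with randomised dimensions.
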(fn `GenerateNextMovementBehaviour`
  (locals (speed :type "Float (double-precision)") (behavior :type Integer) (leftOrRight :type "Float (double-precision)"))
  (bind __simulator (`self._simulator`))
  (bind __simulator_2 (`self._simulator`))
  (bind __simulator_3 (`self._simulator`))
  (bind __simulator_4 (`self._simulator`))
  ;[1 1 1] Generate speed for the next behavior
  (set `local.speed` (`KismetMathLibrary.RandomFloatInRange` (`/Game/DistortionsAndBlurs/Blueprints/AnimatedDroplets/BP_DropletsSimulator.MinSpeed` __simulator) (`/Game/DistortionsAndBlurs/Blueprints/AnimatedDroplets/BP_DropletsSimulator.MaxSpeed` __simulator)))
  ;[1 1 1] Get random value [0..100] which defines next behavior selection
  (set `local.behavior` (`KismetMathLibrary.RandomIntegerInRange` 0 100))
  ;[1 1 1] if behavior value <= linear threshold, then next behavior will be linear, otherwise next behavior will be strafe
  (if (<= (`local.behavior`) (`/Game/DistortionsAndBlurs/Blueprints/AnimatedDroplets/BP_DropletsSimulator.LinearMovementPercent` (`self._simulator`)))
    ;[1 1 1] Configure next linear behavior
    (bind _returnvalue (`|GenericCreateObject` "/Game/DistortionsAndBlurs/Blueprints/AnimatedDroplets/BP_LinearDropletMover.BP_LinearDropletMover_C" self))
    (`/Game/DistortionsAndBlurs/Blueprints/AnimatedDroplets/BP_LinearDropletMover.Init` _returnvalue (`self._simulator`) (`self.Position`) (`self.Direction`) (`KismetMathLibrary.RandomFloatInRange` (`/Game/DistortionsAndBlurs/Blueprints/AnimatedDroplets/BP_DropletsSimulator.LinearMinDistance` __simulator_3) (`/Game/DistortionsAndBlurs/Blueprints/AnimatedDroplets/BP_DropletsSimulator.LinearMaxDistance` __simulator_3)) (`local.speed`))
    (set `self._mover` _returnvalue)
    (else
      ;[1 1 1] Choose direction of the strafe behavior (left or right)
      (set `local.leftOrRight` (`KismetMathLibrary.SelectFloat` 1.0 -1.0 (> (`local.behavior`) (+ (`/Game/DistortionsAndBlurs/Blueprints/AnimatedDroplets/BP_DropletsSimulator.LinearMovementPercent` (`self._simulator`)) (/ (- 100 (`/Game/DistortionsAndBlurs/Blueprints/AnimatedDroplets/BP_DropletsSimulator.LinearMovementPercent` (`self._simulator`))) 2)))))
      ;[1 1 1] Configure next strafe behavior
      (bind _returnvalue_2 (`|GenericCreateObject` "/Game/DistortionsAndBlurs/Blueprints/AnimatedDroplets/BP_StrafeDropletMover.BP_StrafeDropletMover_C" self))
      (`/Game/DistortionsAndBlurs/Blueprints/AnimatedDroplets/BP_StrafeDropletMover.Init` _returnvalue_2 (`self._simulator`) (`self.Position`) (`self.Direction`) (`KismetMathLibrary.MakeVector2D` (* (`KismetMathLibrary.RandomFloatInRange` (`/Game/DistortionsAndBlurs/Blueprints/AnimatedDroplets/BP_DropletsSimulator.StrafeMinWidth` __simulator_2) (`/Game/DistortionsAndBlurs/Blueprints/AnimatedDroplets/BP_DropletsSimulator.StrafeMaxWidth` __simulator_2)) (`local.leftOrRight`)) (`KismetMathLibrary.RandomFloatInRange` (`/Game/DistortionsAndBlurs/Blueprints/AnimatedDroplets/BP_DropletsSimulator.StrafeMinHeight` __simulator_4) (`/Game/DistortionsAndBlurs/Blueprints/AnimatedDroplets/BP_DropletsSimulator.StrafeMaxHeight` __simulator_4))) (`local.speed`) (`/Game/DistortionsAndBlurs/Blueprints/AnimatedDroplets/BP_DropletsSimulator.StrafeSpeedSlowdownFactor` (`self._simulator`)))
      (set `self._mover` _returnvalue_2))))

(fn `Init`
  (params (simulator :type "/Game/DistortionsAndBlurs/Blueprints/AnimatedDroplets/BP_DropletsSimulator Object Reference") (position :type "Vector2D Structure") (direction :type "Vector2D Structure") (size :type "Vector2D Structure"))
  (set `self._simulator` simulator)
  (set `self.Position` position)
  (set `self.Direction` direction)
  (set `self.Size` size)
  (set `self.Active` true)
  (`self.GenerateNextMovementBehaviour`))

(fn `Move`
  (params (deltaTime :type "Float (double-precision)"))
  (locals (finishedMovement :type Boolean))
  (bind (_finishedmovement _position _direction) (`/Game/DistortionsAndBlurs/Blueprints/AnimatedDroplets/BP_DropletMover.Move` (`self._mover`) deltaTime))
  (set `self.Position` _position)
  (set `self.Direction` _direction)
  (if _finishedmovement
    (`self.GenerateNextMovementBehaviour`))
  (return))