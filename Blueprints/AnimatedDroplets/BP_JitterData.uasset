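; BP_JitterData holds per-instance jitter parameters for the animated droplets and computes their wobble over time.
; Init draws random macro and micro amplitudes from the Simulator's ranges and copies its two frequencies.
; CalcJitter sums two sine waves at those frequencies and amplitudes, layering macro and micro oscillation into one offset value for a given time.
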(fn `CalcJitter`
  (params (time :type "Float (double-precision)"))
  (returns (result :type "Float (double-precision)"))
  (return (+ (* (`KismetMathLibrary.Sin` (* time (`self._microJitterTimeCoeff`))) (`self._microJitter`)) (* (`KismetMathLibrary.Sin` (* time (`self._macroJitterTimeCoeff`))) (`self._macroJitter`)))))

(fn `Init`
  (params (simulator :type "/Game/DistortionsAndBlurs/Blueprints/AnimatedDroplets/BP_DropletsSimulator Object Reference"))
  (set `self._macroJitter` (`KismetMathLibrary.RandomFloatInRange` (`/Game/DistortionsAndBlurs/Blueprints/AnimatedDroplets/BP_DropletsSimulator.MacroJitterAmplitudeMin` simulator) (`/Game/DistortionsAndBlurs/Blueprints/AnimatedDroplets/BP_DropletsSimulator.MacroJitterAmplitudeMax` simulator)))
  (set `self._microJitter` (`KismetMathLibrary.RandomFloatInRange` (`/Game/DistortionsAndBlurs/Blueprints/AnimatedDroplets/BP_DropletsSimulator.MicroJitterAmplitudeMin` simulator) (`/Game/DistortionsAndBlurs/Blueprints/AnimatedDroplets/BP_DropletsSimulator.MicroJitterAmplitudeMax` simulator)))
  (set `self._macroJitterTimeCoeff` (`/Game/DistortionsAndBlurs/Blueprints/AnimatedDroplets/BP_DropletsSimulator.MacroJitterFrequency` simulator))
  (set `self._microJitterTimeCoeff` (`/Game/DistortionsAndBlurs/Blueprints/AnimatedDroplets/BP_DropletsSimulator.MicroJitterFrequency` simulator)))