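; Droplet mover that carries an animated droplet forward while strafing it sideways along an S-curve within a block.
; Init stores the block size, speed and slowdown, and derives the perpendicular to the initial direction.
; Each move advances distance at a sine-eased speed that changes most mid-block, then maps it to an arctangent lateral offset.
; The curve's analytic derivative sets heading, and the move reports completion at block length.
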(fn `Init`
  (params (simulator :type "/Game/DistortionsAndBlurs/Blueprints/AnimatedDroplets/BP_DropletsSimulator Object Reference") (position :type "Vector2D Structure") (direction :type "Vector2D Structure") (blockSize :type "Vector2D Structure") (speed :type "Float (double-precision)") (speedSlowDownCoeff :type "Float (double-precision)"))
  (bind (__initdirection_x __initdirection_y) (`KismetMathLibrary.BreakVector2D` (`self._initDirection`)))
  (`self.BaseInit` simulator position direction)
  (set `self._blockSize` blockSize)
  (set `self._speed` speed)
  (set `self._speedSlowDownCoeff` speedSlowDownCoeff)
  (set `self._initDirectionPerp` (`KismetMathLibrary.MakeVector2D` (* __initdirection_y -1.0) __initdirection_x)))

(fn `MoveImplementation`
  (params (deltaTime :type "Float (double-precision)"))
  (returns (result :type Boolean))
  (locals (coeff :type "Float (double-precision)") (speedCoeff :type "Float (double-precision)") (actualSpeed :type "Float (double-precision)") (t :type "Float (double-precision)") (offset :type "Float (double-precision)") (dtdx :type "Float (double-precision)") (derivative :type "Vector2D Structure"))
  (bind (__blocksize_x __blocksize_y) (`KismetMathLibrary.BreakVector2D` (`self._blockSize`)))
  (bind __blocksize_x_2 (`KismetMathLibrary.BreakVector2D` (`self._blockSize`)))
  (bind (__blocksize_x_3 __blocksize_y_2) (`KismetMathLibrary.BreakVector2D` (`self._blockSize`)))
  (bind (__blocksize_x_4 __blocksize_y_3) (`KismetMathLibrary.BreakVector2D` (`self._blockSize`)))
  (bind _derivative_x (`KismetMathLibrary.BreakVector2D` (`local.derivative`)))
  (bind __blocksize_x_5 (`KismetMathLibrary.BreakVector2D` (`self._blockSize`)))
  (bind _t (`local.t`))
  (bind (_derivative_x_2 _derivative_y) (`KismetMathLibrary.BreakVector2D` (`local.derivative`)))
  (set `local.coeff` (`KismetMathLibrary.FMin` 1.0 (/ (`self._currParamValue`) __blocksize_y)))
  (set `local.speedCoeff` (`KismetMathLibrary.Lerp` 1.0 (`self._speedSlowDownCoeff`) (`KismetMathLibrary.Sin` (`KismetMathLibrary.MultiplyByPi` (`local.coeff`)))))
  (set `local.actualSpeed` (* (`self._speed`) (`local.speedCoeff`)))
  (set `self._currParamValue` (+ (`self._currParamValue`) (* (`local.actualSpeed`) deltaTime)))
  (set `local.t` (- (* (`local.coeff`) 10.0) 5.0))
  (set `local.offset` (* (+ (`KismetMathLibrary.Atan` (`local.t`)) (`KismetMathLibrary.Atan` 5.0)) __blocksize_x_2))
  (set `self._position` (+ (`self._initPosition`) (* (`self._initDirection`) (`self._currParamValue`)) (* (`self._initDirectionPerp`) (`local.offset`))))
  (set `local.dtdx` (/ 10.0 __blocksize_y_3))
  (set `local.derivative` (`KismetMathLibrary.Normal2D` (`KismetMathLibrary.MakeVector2D` 1.0 (* (/ __blocksize_x_5 (+ 1.0 (* _t _t))) (`local.dtdx`)))))
  (set `self._direction` (`KismetMathLibrary.Normal2D` (+ (* (`self._initDirection`) _derivative_x) (* (`self._initDirectionPerp`) _derivative_y))))
  (return (>= (`self._currParamValue`) __blocksize_y_2)))