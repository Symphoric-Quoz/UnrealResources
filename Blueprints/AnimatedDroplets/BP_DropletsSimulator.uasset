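; Simulates animated droplets moving down a surface and renders them into a droplets texture.
; Tick runs a fixed-timestep loop that spawns BP_Droplet objects at random intervals, moves them and removes those past the bottom edge.
; Droplets are stamped onto an internal render target that fades each step, leaving trails.
; A mask material reads this as a heightfield, optionally with a static droplets texture, and draws the output.
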(event EventBeginPlay
  (bind _returnvalue (Rendering|Material|CreateDynamicMaterialInstance "/Game/DistortionsAndBlurs/Materials/MaterialInstances/AnimatedDroplets/MI_CreateDropletsMask.MI_CreateDropletsMask" :!class /Script/Engine.KismetMaterialLibrary))
  (Variables|Default|Set_createDropletsMask _returnvalue)
  (bind _returnvalue_2 (Rendering|Material|CreateDynamicMaterialInstance "/Game/DistortionsAndBlurs/Materials/MaterialInstances/AnimatedDroplets/MI_CreateDropletsMask_Copy.MI_CreateDropletsMask_Copy" :!class /Script/Engine.KismetMaterialLibrary))
  (Variables|Default|Set_createDropletsMaskCopy _returnvalue_2))

(event EventTick
  (params (DeltaSeconds :type Float%20%28single-precision%29))
  (bind _valid (CallFunction|ValidateRenderTarget))
  (if _valid
    (CallFunction|UpdateandRender DeltaSeconds)))

(fn ConstructionScript)

(fn UpdateandRender
  (params (float%20deltaTime :type Float%20%28single-precision%29))
  (Utilities|FlowControl|Sequence
    (:then_0
      (Variables|Default|Set_updateTimer (+ (Variables|Default|Get_updateTimer) float%20deltaTime))
      (Variables|Default|Set_deltaTime (/ 1.0 (Variables|Simulation|GetSimulationFrequency))))
    (:then_1
      ;[1 1 1] Simulate in lockstep specified by SimulationFrequency. Render after simulation as rendering should be in sync.
      (while (>= (Variables|Default|Get_updateTimer) (Variables|Default|Get_deltaTime))
        (Variables|Default|Set_updateTimer (- (Variables|Default|Get_updateTimer) (Variables|Default|Get_deltaTime)))
        (bind _output_get (Variables|Default|Set_gravity (* (Variables|Spawn|GetGravity) -1.0)))
        (Variables|Default|Set_gravity (Math|Vector2D|Normalize2D _output_get))
        (if (Variables|Spawn|GetSpawnEnabled)
          (CallFunction|SpawnDroplets)
          (CallFunction|SimulateDroplets)
          (CallFunction|Render))))))

(fn SpawnDroplets
  ;[1 1 1] If it's time to spawn
  (while (>= (Variables|Default|Get_spawnTimer) (Variables|Default|Get_spawnRate))
    ;[1 1 1] Check if we're not at max number of droplets
    (if (< (Utilities|Array|Length (Variables|Default|Get_droplets)) (Variables|Spawn|GetMaxDroplets))
      ;[1 1 1] Spawn new droplet or skip
      (Utilities|SpawnDroplet
        (:execOut
          _)))
    ;[1 1 1] Update spawn timer
    (Variables|Default|Set_spawnTimer (- (Variables|Default|Get_spawnTimer) (Variables|Default|Get_spawnRate)))
    ;[1 1 1] Choose next spawn rate
    (Variables|Default|Set_spawnRate (Math|Random|RandomFloatinRange (Variables|Spawn|GetSpawnRateMin) (Variables|Spawn|GetSpawnRateMax))))
  ;[1 1 1] Update spawn timer
  (Variables|Default|Set_spawnTimer (+ (Variables|Default|Get_spawnTimer) (Variables|Default|Get_deltaTime))))

(fn SimulateDroplets
  (for _index (range 0 (Utilities|Array|LastIndex (Variables|Default|Get_droplets)))
    (bind _output_get (LocalVariables|Setdroplet (Utilities|Array|Get(acopy) (Variables|Default|Get_droplets) _index)))
    (Default|Move _output_get (Variables|Default|Get_deltaTime))
    (bind _remove (Utilities|ShouldRemoveDroplet _output_get)
      (:execOut
        (if _remove
          (Utilities|Array|Add (LocalVariables|GetdeleteIndices) _index)))))
  (LocalVariables|Setindex (Utilities|Array|LastIndex (LocalVariables|GetdeleteIndices)))
  (while (>= (LocalVariables|Getindex) 0)
    (Utilities|Array|RemoveIndex (Variables|Default|Get_droplets) (Utilities|Array|Get(acopy) (LocalVariables|GetdeleteIndices) (LocalVariables|Getindex)))
    (Math|Integer|DecrementInt (LocalVariables|Getindex))))

(fn Render
  (bind _shiftuv (Variables|StaticDroplets|GetShiftUV))
  (bind _tileuv (Variables|StaticDroplets|GetTileUV))
  ;[1 1 1] Fade out droplets
  (Utilities|BeginDrawing (Variables|Default|Get_dropletsRT) (LocalVariables|Getcanvas) (LocalVariables|Getsize) (LocalVariables|Getcontext)
    (:out
      (Canvas|DrawTexture :self (LocalVariables|Getcanvas) :ScreenSize (LocalVariables|Getsize) :RenderColor (Utilities|Struct|MakeLinearColor 0.0 0.0 0.0 (Variables|Simulation|GetDropletsFadeRate)))
      ;[1 1 1] Draw current droplets
      (for _array_element (Variables|Default|Get_droplets)
        (Canvas|DrawTexture (LocalVariables|Getcanvas) "/Game/DistortionsAndBlurs/Textures/T_Droplet_0.T_Droplet_0" (Variables|/Game/DistortionsAndBlurs/Blueprints/AnimatedDroplets/BP_Droplet.BP_Droplet_C|GetPosition _array_element) (Variables|/Game/DistortionsAndBlurs/Blueprints/AnimatedDroplets/BP_Droplet.BP_Droplet_C|GetSize _array_element) "(X=0.000000,Y=0.000000)" "(X=1.000000,Y=-1.000000)" "(R=1.000000,G=1.000000,B=1.000000,A=1.000000)" "BLEND_Translucent" (Class|KismetMathLibrary|DegAtan2 (.x (Variables|/Game/DistortionsAndBlurs/Blueprints/AnimatedDroplets/BP_Droplet.BP_Droplet_C|GetDirection _array_element)) (* (.y (Variables|/Game/DistortionsAndBlurs/Blueprints/AnimatedDroplets/BP_Droplet.BP_Droplet_C|GetDirection _array_element)) -1.0)) "(X=0.500,Y=0.500)"))
      (Rendering|EndDrawCanvastoRenderTarget (LocalVariables|Getcontext))
      ;[1 1 1] Set creation material instance parameters
      (Utilities|IsValid (Variables|StaticDroplets|GetStaticDropletsTexture)
        (:Is%20Valid
          (LocalVariables|Setmid (Variables|Default|Get_createDropletsMaskCopy))
          (Rendering|Material|SetTextureParameterValue (LocalVariables|Getmid) "StaticDroplets" (Variables|StaticDroplets|GetStaticDropletsTexture)))
        (:Is%20Not%20Valid
          (LocalVariables|Setmid (Variables|Default|Get_createDropletsMask))))
      (Rendering|Material|SetVectorParameterValue (LocalVariables|Getmid) "UVEdit" (Utilities|Struct|MakeLinearColor (.x _shiftuv) (.y _shiftuv) (.x _tileuv) (.y _tileuv)) :!class /Script/Engine.MaterialInstanceDynamic)
      (Rendering|Material|SetTextureParameterValue (LocalVariables|Getmid) "Heightfield" (Variables|Default|Get_dropletsRT))
      (Rendering|Material|SetScalarParameterValue (LocalVariables|Getmid) "HeightScale" (Variables|Droplets|GetHeghtScale) :!class /Script/Engine.MaterialInstanceDynamic)
      (Rendering|Material|SetScalarParameterValue (LocalVariables|Getmid) "TexelSizeX" (/ 1.0 (Math|Conversions|ToFloat(Integer) (Variables|Default|Get_width))) :!class /Script/Engine.MaterialInstanceDynamic)
      (Rendering|Material|SetScalarParameterValue (LocalVariables|Getmid) "TexelSizeY" (/ 1.0 (Math|Conversions|ToFloat(Integer) (Variables|Default|Get_height))) :!class /Script/Engine.MaterialInstanceDynamic)
      ;[1 1 1] Call final composition material
      (Rendering|ClearRenderTarget2D (Variables|ResultRenderTarget|GetDropletsTexture) "(R=0.000000,G=0.000000,B=0.000000,A=1.000000)")
      (Utilities|BeginDrawing (Variables|ResultRenderTarget|GetDropletsTexture) (LocalVariables|Getcanvas) (LocalVariables|Getsize) (LocalVariables|Getcontext)
        (:out
          (Canvas|DrawMaterial :self (LocalVariables|Getcanvas) :RenderMaterial (LocalVariables|Getmid) :ScreenSize (LocalVariables|Getsize))
          (Rendering|EndDrawCanvastoRenderTarget (LocalVariables|Getcontext)))))))

(fn ValidateRenderTarget
  (bind _dropletstexture (Variables|ResultRenderTarget|GetDropletsTexture))
  (Utilities|IsValid (Variables|ResultRenderTarget|GetDropletsTexture)
    (:Is%20Valid
      (Variables|Default|Set_width (Variables|/Script/Engine.TextureRenderTarget2D|GetSizeX _dropletstexture))
      (Variables|Default|Set_height (Variables|/Script/Engine.TextureRenderTarget2D|GetSizeY _dropletstexture))
      (Utilities|IsValid (Variables|Default|Get_dropletsRT)
        (:Is%20Valid
          (if (|((sizeX!=width)||(sizeY!=height)) (Variables|/Script/Engine.TextureRenderTarget2D|GetSizeX (Variables|Default|Get_dropletsRT)) (Variables|Default|Get_width) (Variables|/Script/Engine.TextureRenderTarget2D|GetSizeY (Variables|Default|Get_dropletsRT)) (Variables|Default|Get_height))
            (bind _returnvalue (Rendering|CreateRenderTarget2D (Variables|Default|Get_width) (Variables|Default|Get_height) :!label _label))
            (bind _output_get (Variables|Default|Set_dropletsRT _returnvalue))
            (Rendering|ClearRenderTarget2D _output_get)))
        (:Is%20Not%20Valid
          (goto _label)))
      (return true))
    (:Is%20Not%20Valid
      (return false))))

(fn Reset
  (Utilities|Array|Clear (Variables|Default|Get_droplets))
  (Variables|Default|Set_updateTimer 0.0)
  (Variables|Default|Set_spawnRate 0.0)
  (Variables|Default|Set_spawnTimer 0.0)
  (Rendering|ClearRenderTarget2D (Variables|Default|Get_dropletsRT)))