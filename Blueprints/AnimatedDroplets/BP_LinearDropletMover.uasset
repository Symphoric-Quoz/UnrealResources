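; BP_LinearDropletMover is a droplet mover that moves an animated droplet in a straight 2D line at constant speed.
; Init passes simulator, position and direction to the base init, then stores the target distance and speed.
; MoveImplementation advances the position along the direction, scaled by delta time, and accumulates travelled distance, returning true once the target distance is reached.
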(fn `Init`
  (params (simulator :type "/Game/DistortionsAndBlurs/Blueprints/AnimatedDroplets/BP_DropletsSimulator Object Reference") (position :type "Vector2D Structure") (direction :type "Vector2D Structure") (targetDistance :type "Float (double-precision)") (speed :type "Float (double-precision)"))
  (`self.BaseInit` simulator position direction)
  (set `self._targetDistance` targetDistance)
  (set `self._speed` speed))

(fn `MoveImplementation`
  (params (deltaTime :type "Float (double-precision)"))
  (returns (result :type Boolean))
  (locals (positionOffset :type "Vector2D Structure"))
  (bind _output_get (set `local.positionOffset` (* (`self._direction`) (* deltaTime (`self._speed`)))))
  (set `self._position` (+ _output_get (`self._position`)))
  (set `self._travelledDistance` (+ (`self._travelledDistance`) (`KismetMathLibrary.VSize2D` (`local.positionOffset`))))
  (return (>= (`self._travelledDistance`) (`self._targetDistance`))))