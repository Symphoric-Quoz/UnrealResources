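; BP_DropletMover is a base object that moves an animated droplet, storing its initial and current position and direction.
; Init creates a BP_JitterData from the supplied simulator.
; Move advances a timer, calls the overridable MoveImplementation (which returns unfinished by default), then offsets the returned position perpendicular to the direction by time-based jitter.
; The jitter affects only the returned position, leaving the stored position unchanged.
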(fn `BaseInit`
  (params (simulator :type "/Game/DistortionsAndBlurs/Blueprints/AnimatedDroplets/BP_DropletsSimulator Object Reference") (position :type "Vector2D Structure") (direction :type "Vector2D Structure"))
  (set `self._simulator` simulator)
  (bind _output_get (set `self._initPosition` position))
  (set `self._position` _output_get)
  (bind _output_get_2 (set `self._initDirection` direction))
  (set `self._direction` _output_get_2)
  (bind _returnvalue (`|GenericCreateObject` "/Game/DistortionsAndBlurs/Blueprints/AnimatedDroplets/BP_JitterData.BP_JitterData_C" self))
  (bind _output_get_3 (set `self._jitterData` _returnvalue))
  (`/Game/DistortionsAndBlurs/Blueprints/AnimatedDroplets/BP_JitterData.Init` _output_get_3 (`self._simulator`))
  (return))

(fn `Move`
  (params (deltaTime :type "Float (double-precision)"))
  (returns (finishedMovement :type Boolean) (position :type "Vector2D Structure") (direction :type "Vector2D Structure"))
  (locals (jitterOffset :type "Vector2D Structure"))
  (bind (__direction_x __direction_y) (`KismetMathLibrary.BreakVector2D` (`self._direction`)))
  ;[1 1 1] Update timer
  (set `self._timer` (+ deltaTime (`self._timer`)))
  ;[1 1 1] Call virtual move function
  (bind _result (`self.MoveImplementation` deltaTime))
  ;[1 1 1] Calc jitter
  (bind _result_2 (`/Game/DistortionsAndBlurs/Blueprints/AnimatedDroplets/BP_JitterData.CalcJitter` (`self._jitterData`) (`self._timer`)))
  (bind _output_get (set `local.jitterOffset` (`KismetMathLibrary.MakeVector2D` (* _result_2 -1.0 __direction_y) (* __direction_x _result_2))))
  ;[1 1 1] Return position and direction
  (return _result (+ _output_get (`self._position`)) (`self._direction`)))

(fn `MoveImplementation`
  (params (deltaTime :type "Float (double-precision)"))
  (returns (result :type Boolean))
  (return false))